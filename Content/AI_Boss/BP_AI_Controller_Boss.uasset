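; AI controller for a boss that runs the boss behavior tree and manages the boss health bar on screen.
; BeginPlay starts BT_AI_Boss.
; ActivateBossCombat creates the WB_Boss_HealthBar widget and adds it to the viewport, and DeactivateBossCombat removes it and clears the reference.
; While that widget is valid, Tick polls Health over MaxHealth to set the bar's fill.
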(event `self.ReceiveBeginPlay`
  (`self.RunBehaviorTree` "/Game/AI_Boss/BT_AI_Boss.BT_AI_Boss"))

(event `Activate Boss Combat`
  (bind _returnvalue (`|CreateWidget` "/Game/UI/WB_Boss_HealthBar.WB_Boss_HealthBar_C"))
  (bind _output_get (set `self.Boss_Health_Bar_Widget` _returnvalue))
  (`UserWidget.AddToViewport` _output_get 0))

(event `Deactivate Boss Combat`
  (`Widget.RemoveFromParent` (`self.Boss_Health_Bar_Widget`))
  (set `self.Boss_Health_Bar_Widget` null))

(event `self.ReceiveTick`
  (params (DeltaSeconds :type "Float (single-precision)"))
  (bind _boss_health_bar_widget (`self.Boss_Health_Bar_Widget`)
    (:`then`
      (`ProgressBar.SetPercent` (`/Game/UI/WB_Boss_HealthBar.HealthBar` _boss_health_bar_widget) (/ (`self.Health`) (`self.Max Health`))))
    (:`else`)))

(fn `UserConstructionScript`
  (`parent.UserConstructionScript`))