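; Stat component for the player, Trooper and Boss that tracks health, plus stamina, XP and level for the player.
; BeginPlay waits a tick, casts the owner to set CharacterType, initializes its widgets and calls IncreaseLevel for the player.
; DecreaseHealth uses that type to select the widget and returns whether health is depleted.
; Other functions update the player HUD directly; leveling raises MaxXP, resets XP and plays sounds.
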(event `self.ReceiveBeginPlay`
  (`KismetSystemLibrary.DelayUntilNextTick`)
  (bind _asbp_third_person_character (cast `/Game/ThirdPerson/Blueprints/BP_ThirdPersonCharacter` (`self.GetOwner`))
    (:`then`
      (set `self.Player Character` _asbp_third_person_character)
      (set `self.Is Player` true)
      (`ProgressBar.SetPercent` (`/Game/UI/WB_HUD.StaminaBar` (`/Game/ThirdPerson/Blueprints/BP_ThirdPersonCharacter.Hud Widget` (`self.Player Character`))) (/ (`self.Current Stamina `) (`self.Max Stamina`)))
      (set `self.Character Type` "NewEnumerator0"))
    (:`CastFailed`
      (bind _asbp_ai_boss (cast `/Game/AI_Boss/BP_AI_Boss` (`self.GetOwner`))
        (:`then`
          (set `self. BP AI Boss` _asbp_ai_boss)
          (set `self.Is Player` false)
          (set `self.Character Type` "NewEnumerator2"))
        (:`CastFailed`
          (bind _asbp_trooper_1 (cast `/Game/AI_Trooper/BP_Trooper1` (`self.GetOwner`)))
          (set `self.BP Trooper 1` _asbp_trooper_1)
          (set `self.Character Type` "NewEnumerator1")))))
  (`ProgressBar.SetPercent` (select `/Game/Blueprints/E_Character_Types` (`self.Character Type`) :`NewEnumerator0` (`/Game/UI/WB_HUD.HealthBar` (`/Game/ThirdPerson/Blueprints/BP_ThirdPersonCharacter.Hud Widget` (`self.Player Character`))) :`NewEnumerator1` (`/Game/UI/WB_Dummy_Healthbar.HealthBar` (`/Game/AI_Trooper/BP_Trooper1.Health Bar UI` (`self.BP Trooper 1`))) :`NewEnumerator2` (`/Game/UI/WB_Dummy_Healthbar.HealthBar` (`/Game/AI_Boss/BP_AI_Boss.Health Bar UI` (`self. BP AI Boss`)))) (/ (`self.Current Health`) (`self.Max Health`)))
  (`TextBlock.SetText` (select `/Game/Blueprints/E_Character_Types` (`self.Character Type`) :`NewEnumerator0` (`/Game/UI/WB_HUD.HealthText` (`/Game/ThirdPerson/Blueprints/BP_ThirdPersonCharacter.Hud Widget` (`self.Player Character`))) :`NewEnumerator1` (`/Game/UI/WB_Dummy_Healthbar.HealthText` (`/Game/AI_Trooper/BP_Trooper1.Health Bar UI` (`self.BP Trooper 1`))) :`NewEnumerator2` (`/Game/UI/WB_Dummy_Healthbar.HealthText` (`/Game/AI_Boss/BP_AI_Boss.Health Bar UI` (`self. BP AI Boss`)))) (`KismetTextLibrary.Conv_DoubleToText` (`self.Current Health`) "HalfToEven"))
  (if (`self.Is Player`)
    (`self.Increase Level` 1)
    (`ProgressBar.SetPercent` (`/Game/UI/WB_HUD.XPBar` (`/Game/ThirdPerson/Blueprints/BP_ThirdPersonCharacter.Hud Widget` (`self.Player Character`))) (/ (`self.XP`) (`self.Max XP`)))
    (`TextBlock.SetText` (`/Game/UI/WB_HUD.XPText` (`/Game/ThirdPerson/Blueprints/BP_ThirdPersonCharacter.Hud Widget` (`self.Player Character`))) (`|FormatText` "{Current XP} / {Max XP}" (`self.XP`) (`self.Max XP`)))
    (`TextBlock.SetText` (`/Game/UI/WB_HUD.LevelText` (`/Game/ThirdPerson/Blueprints/BP_ThirdPersonCharacter.Hud Widget` (`self.Player Character`))) (`KismetTextLibrary.Conv_IntToText` (`self.Level`)))))

(fn `Decrease Health`
  (params (Damage :type "Float (double-precision)"))
  (returns (`Is Player Dead` :type Boolean))
  (if (not (<= (`self.Current Health`) 0.0))
    (bind _output_get (set `self.Current Health` (- (`self.Current Health`) Damage)))
    (`ProgressBar.SetPercent` (select `/Game/Blueprints/E_Character_Types` (`self.Character Type`) :`NewEnumerator0` (`/Game/UI/WB_HUD.HealthBar` (`/Game/ThirdPerson/Blueprints/BP_ThirdPersonCharacter.Hud Widget` (`self.Player Character`))) :`NewEnumerator1` (`/Game/UI/WB_Dummy_Healthbar.HealthBar` (`/Game/AI_Trooper/BP_Trooper1.Health Bar UI` (`self.BP Trooper 1`))) :`NewEnumerator2` (`/Game/UI/WB_Dummy_Healthbar.HealthBar` (`/Game/AI_Boss/BP_AI_Boss.Health Bar UI` (`self. BP AI Boss`)))) (/ _output_get (`self.Max Health`)))
    (`TextBlock.SetText` (select `/Game/Blueprints/E_Character_Types` (`self.Character Type`) :`NewEnumerator0` (`/Game/UI/WB_HUD.HealthText` (`/Game/ThirdPerson/Blueprints/BP_ThirdPersonCharacter.Hud Widget` (`self.Player Character`))) :`NewEnumerator1` (`/Game/UI/WB_Dummy_Healthbar.HealthText` (`/Game/AI_Trooper/BP_Trooper1.Health Bar UI` (`self.BP Trooper 1`))) :`NewEnumerator2` (`/Game/UI/WB_Dummy_Healthbar.HealthText` (`/Game/AI_Boss/BP_AI_Boss.Health Bar UI` (`self. BP AI Boss`)))) (`KismetTextLibrary.Conv_DoubleToText` (`self.Current Health`) "HalfToEven"))
    (if (<= (`self.Current Health`) 0.0)
      _
      (else
        (return false))))
  (return true))

(fn `Decrease Stamina`
  (params (`Stamina Depleted` :type "Float (double-precision)"))
  (returns (`Not Stamina Left` :type Boolean))
  (if (not (<= (`self.Current Stamina `) 0.0))
    (set `self.Current Stamina ` (- (`self.Current Stamina `) `Stamina Depleted`))
    (`ProgressBar.SetPercent` (`/Game/UI/WB_HUD.StaminaBar` (`/Game/ThirdPerson/Blueprints/BP_ThirdPersonCharacter.Hud Widget` (`self.Player Character`))) (/ (`self.Current Stamina `) (`self.Max Stamina`)))
    (if (<= (`self.Current Stamina `) 0.0)
      _
      (else
        (return false))))
  (return true))

(fn `Incease Health`
  (params (`Added Health` :type "Float (double-precision)"))
  (bind _hud_widget (`/Game/ThirdPerson/Blueprints/BP_ThirdPersonCharacter.Hud Widget` (`self.Player Character`)))
  (set `self.Current Health` (+ (`self.Current Health`) `Added Health`))
  (if (> (`self.Current Health`) (`self.Max Health`))
    (set `self.Current Health` (`self.Max Health`)))
  (`ProgressBar.SetPercent` (`/Game/UI/WB_HUD.HealthBar` _hud_widget) (/ (`self.Current Health`) (`self.Max Health`)))
  (`TextBlock.SetText` (`/Game/UI/WB_HUD.HealthText` _hud_widget) (`KismetTextLibrary.Conv_DoubleToText` (`self.Current Health`) "HalfToEven")))

(fn `Increase Level`
  (params (`Added Level` :type Integer))
  (set `self.Level` (+ (`self.Level`) `Added Level`))
  (set `self.Max XP` (+ (`self.Max XP`) 150.0))
  (set `self.XP` 0.0)
  (`TextBlock.SetText` (`/Game/UI/WB_HUD.LevelText` (`/Game/ThirdPerson/Blueprints/BP_ThirdPersonCharacter.Hud Widget` (`self.Player Character`))) (`KismetTextLibrary.Conv_IntToText` (`self.Level`)))
  (`GameplayStatics.PlaySound2D` "/Game/Audio/UI/LevelUp1.LevelUp1" 1.0 1.0 0.0 null null)
  (`GameplayStatics.PlaySound2D` "/Game/Audio/UI/LevelUp2.LevelUp2" 1.0 1.0 0.0 null null))

(fn `Increase Max Health`
  (params (`Health Increasing` :type "Float (double-precision)"))
  (bind _hud_widget (`/Game/ThirdPerson/Blueprints/BP_ThirdPersonCharacter.Hud Widget` (`self.Player Character`)))
  (set `self.Max Health` (+ (`self.Max Health`) `Health Increasing`))
  (`ProgressBar.SetPercent` (`/Game/UI/WB_HUD.HealthBar` _hud_widget) (/ (`self.Current Health`) (`self.Max Health`)))
  (`TextBlock.SetText` (`/Game/UI/WB_HUD.HealthText` _hud_widget) (`KismetTextLibrary.Conv_DoubleToText` (`self.Current Health`) "HalfToEven")))

(fn `Increase Max Stamina`
  (params (`Added Stamina` :type "Float (double-precision)"))
  (bind _output_get (set `self.Max Stamina` (+ (`self.Max Stamina`) `Added Stamina`)))
  (set `self.Current Stamina ` _output_get)
  (`ProgressBar.SetPercent` (`/Game/UI/WB_HUD.StaminaBar` (`/Game/ThirdPerson/Blueprints/BP_ThirdPersonCharacter.Hud Widget` (`self.Player Character`))) (/ (`self.Current Stamina `) (`self.Max Stamina`))))

(fn `Increase Stamina`
  (params (`Added Stamina` :type "Float (double-precision)"))
  (set `self.Current Stamina ` (+ (`self.Max Stamina`) `Added Stamina`))
  (if (> (`self.Current Stamina `) (`self.Max Stamina`))
    (set `self.Current Stamina ` (`self.Max Stamina`)))
  (`ProgressBar.SetPercent` (`/Game/UI/WB_HUD.StaminaBar` (`/Game/ThirdPerson/Blueprints/BP_ThirdPersonCharacter.Hud Widget` (`self.Player Character`))) (/ (`self.Current Stamina `) (`self.Max Stamina`))))

(fn `Increase XP`
  (params (`Addded XP` :type "Float (double-precision)"))
  (set `self.XP` (+ (`self.XP`) `Addded XP`))
  (if (>= (`self.XP`) (`self.Max XP`))
    (`self.Increase Level` 1))
  (`ProgressBar.SetPercent` (`/Game/UI/WB_HUD.XPBar` (`/Game/ThirdPerson/Blueprints/BP_ThirdPersonCharacter.Hud Widget` (`self.Player Character`))) (/ (`self.XP`) (`self.Max XP`)))
  (`TextBlock.SetText` (`/Game/UI/WB_HUD.XPText` (`/Game/ThirdPerson/Blueprints/BP_ThirdPersonCharacter.Hud Widget` (`self.Player Character`))) (`|FormatText` "{Current XP} / {Max XP}" (`self.XP`) (`self.Max XP`))))