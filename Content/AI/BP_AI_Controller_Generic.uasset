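; Generic AI controller that runs the BT_AI behavior tree and feeds sight and hearing perception into its blackboard.
; Sight sets Target Actor; lost sight or any non-sight stimulus clears it.
; Hearing writes Investigation Location and enables the investigation icon on Trooper1 or Boss pawns.
; Sight handling also casts itself to the boss controller to toggle boss combat.
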(event `self.ReceiveBeginPlay`
  (`self.RunBehaviorTree` "/Game/AI/BT_AI.BT_AI"))

(event `self.AIPerception.OnTargetPerceptionUpdated`
  (params (Actor :type "Actor Object Reference") (Stimulus :type "AIStimulus Structure"))
  ;[0.05127 0.05127 0.05127] Detect and Chase
  (`self.Sight Detection` Actor Stimulus)
  (`self.Hearing Detection` Actor Stimulus))

(fn `Hearing Detection`
  (params (Actor :type "Actor Object Reference") (Stimulus :type "AIStimulus Structure"))
  (bind _returnvalue (`self.K2_GetPawn`))
  (bind _returnvalue_2 (`AIPerceptionSystem.GetSenseClassForStimulus` Stimulus))
  (if (== _returnvalue_2 "/Script/AIModule.AISense_Hearing")
    (`BlackboardComponent.SetValueAsVector` (`AIBlueprintHelperLibrary.GetBlackboard` null) "Investigation Location" (`.StimulusLocation` (break `AIStimulus` Stimulus)))
    (`|ExecutionSequence`
      (:`then_0`
        (bind _asbp_trooper_1 (cast `/Game/AI_Trooper/BP_Trooper1` _returnvalue))
        (`/Game/AI_Trooper/BP_Trooper1.Enable Investigation Icon` _asbp_trooper_1))
      (:`then_1`
        (bind _asbp_ai_boss (cast `/Game/AI_Boss/BP_AI_Boss` _returnvalue))
        (`/Game/AI_Boss/BP_AI_Boss.Enable Investigation Icon` _asbp_ai_boss)))))

(fn `Sight Detection`
  (params (Actor :type "Actor Object Reference") (Stimulus :type "AIStimulus Structure"))
  ;[0.05127 0.05127 0.05127] Detect and Chase
  (bind _returnvalue (`AIPerceptionSystem.GetSenseClassForStimulus` Stimulus))
  (if (== _returnvalue "/Script/AIModule.AISense_Sight")
    (if (`.bSuccessfullySensed` (break `AIStimulus` Stimulus))
      (`BlackboardComponent.SetValueAsObject` (`AIBlueprintHelperLibrary.GetBlackboard` null) "Target Actor" Actor)
      (bind _asbp_ai_controller_boss (cast `/Game/AI_Boss/BP_AI_Controller_Boss` self))
      (`/Game/AI_Boss/BP_AI_Controller_Boss.Activate Boss Combat` _asbp_ai_controller_boss)
      (else
        (`BlackboardComponent.SetValueAsObject` (`AIBlueprintHelperLibrary.GetBlackboard` null) "Target Actor" null :!label _label)
        (bind _asbp_ai_controller_boss_2 (cast `/Game/AI_Boss/BP_AI_Controller_Boss` self))
        (`/Game/AI_Boss/BP_AI_Controller_Boss.Deactivate Boss Combat` _asbp_ai_controller_boss_2)))
    (else
      (goto _label))))

(fn `UserConstructionScript`)